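; BP_TestDummy is a combat test dummy character that can be locked onto and receive damage.
; It calls InitializeCharacter on BeginPlay and shows or hides its lock-on widget when targeted.
; Damage and targeting checks both query the StateManager and refuse only in the Dead state, while the desired rotation is always zero.
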(event `self.ReceiveBeginPlay`
  (`self.InitializeCharacter`))

(event `/Game/CombatSystem/Blueprints/Interfaces/BPI_Targeting.OnTargeted`
  (params (`bIsTargeted?` :type Boolean))
  (`SceneComponent.SetVisibility` (`self.LockOnWidget`) `bIsTargeted?` false))

(fn `CanBeTargeted?`
  (returns (ReturnValue :type Boolean))
  (return (not (`/Game/CombatSystem/Blueprints/Components/BP_StateManager.IsCurrentStateEqualToAny?` (`self.StateManager`) (struct :`GameplayTags` (struct :`(TagName` "Character.State.Dead")))))))

(fn `CanReceiveDamage?`
  (returns (ReturnValue :type Boolean))
  (return (!= (`/Game/CombatSystem/Blueprints/Components/BP_StateManager.GetCurrentState` (`self.StateManager`)) (struct :`TagName` "Character.State.Dead"))))

(fn `GetDesiredRotation`
  (returns (ReturnValue :type "Rotator Structure"))
  (return))

(fn `UserConstructionScript`
  (`parent.UserConstructionScript`))