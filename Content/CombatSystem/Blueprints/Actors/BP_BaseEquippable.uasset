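; BP_BaseEquippable is a base actor in the combat system for items a character can equip.
; It supports static or skeletal visuals, with GetItemMesh returning the static mesh component if it has a mesh assigned, otherwise the skeletal one.
; Equipping sets the equipped flag and snaps the item to the attach socket on the owning Character's mesh.
; Unequipping only clears the flag and does not detach the item.
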(fn `AttachActor`
  (params (SocketName :type Name))
  (`self.K2_AttachToComponent` (`Character.Mesh` (cast `Character` (`self.GetOwner`) :!pure true)) SocketName "SnapToTarget" "SnapToTarget" "SnapToTarget"))

(fn `GetItemMesh`
  (returns (ReturnValue :type "PrimitiveComponent Object Reference"))
  (bind _itemmesh (`self.ItemMesh`))
  (`/Engine/EditorBlueprintResources/StandardMacros.IsValid` (`StaticMeshComponent.StaticMesh` _itemmesh)
    (:`Is Valid`
      (return _itemmesh))
    (:`Is Not Valid`
      (return (`self.ItemSkeletalMesh`)))))

(fn `IsEquipped?`
  (returns (ReturnValue :type Boolean))
  (return (`self.bIsEquipped?`)))

(fn `OnEquipped`
  (set `self.bIsEquipped?` true)
  (`self.AttachActor` (`self.AttachSocketName`)))

(fn `OnUnequipped`
  (if (`self.bIsEquipped?`)
    (set `self.bIsEquipped?` false)))

(fn `SetIsEquipped`
  (params (`IsEquipped?` :type Boolean))
  (set `self.bIsEquipped?` `IsEquipped?`))

(fn `UserConstructionScript`)