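; BP_MasterPose is an equippable armor item whose skeletal mesh follows the animation of the character wearing it.
; AttachActor snaps the item mesh to a socket on the owning Character's mesh and sets that mesh as leader pose component, so the piece deforms with the body.
; Equip and unequip extend the parent logic, adding or subtracting ArmorValue on a stat in the owner's BP_StatsComponent.
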(fn `AttachActor`
  (params (SocketName :type Name))
  (bind _itemskeletalmesh (`self.ItemSkeletalMesh`))
  (`/Engine/EditorBlueprintResources/StandardMacros.IsValid` (`SkeletalMeshComponent.GetSkeletalMeshAsset` _itemskeletalmesh)
    (:`Is Valid`
      (bind _ascharacter (cast `Character` (`self.GetOwner`)))
      (bind _mesh (`Character.Mesh` _ascharacter)
        (:`then`
          (`SceneComponent.K2_AttachToComponent` _itemskeletalmesh _mesh (`local.SocketName`) "SnapToTarget" "SnapToTarget" "SnapToTarget" true)
          (`SkinnedMeshComponent.SetLeaderPoseComponent` (`self.ItemSkeletalMesh`) _mesh false false)
          (return))
        (:`else`)))))

(fn `OnEquipped`
  (`parent.OnEquipped`)
  (`/Game/CombatSystem/Blueprints/Components/BP_StatsComponent.ModifyCurrentStatValue` (`self.GetComponentByClass` (`self.GetOwner`) "/Game/CombatSystem/Blueprints/Components/BP_StatsComponent.BP_StatsComponent_C") "NewEnumerator3" (`self.ArmorValue`) false))

(fn `OnUnequipped`
  (`parent.OnUnequipped`)
  (`/Game/CombatSystem/Blueprints/Components/BP_StatsComponent.ModifyCurrentStatValue` (`self.GetComponentByClass` (`self.GetOwner`) "/Game/CombatSystem/Blueprints/Components/BP_StatsComponent.BP_StatsComponent_C") "NewEnumerator3" (* (`self.ArmorValue`) -1.0) false))

(fn `UserConstructionScript`
  (`parent.UserConstructionScript`))