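; Base dual-wield weapon actor that extends a parent weapon with an off-hand weapon mesh and right-foot attacks.
; On equip and combat toggle, it snaps the off-hand mesh to the owner's hand or stow socket based on combat state.
; Separate collision components for off-hand and foot, switchable by collision part alongside the main weapon, ignore the owner and apply point damage to hit actors that can receive it.
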(event `self.ToggleCombat`
  (params (`bEnableCombat?` :type Boolean))
  (`parent.ToggleCombat` `bEnableCombat?`)
  (`self.AttachOffHandWeapon` (select `bool` `bEnableCombat?` :`false` (`self.SecondWeaponAttachSocket`) :`true` (`self.SecondWeaponHandSocket`))))

(event `self.OffHandWeaponCollisionComponent.OnHit`
  (params (HitResult :type "HitResult Structure"))
  (bind (_bblockinghit _binitialoverlap _time _distance _location _impactpoint _normal _impactnormal _physmat _hitactor) (`GameplayStatics.BreakHitResult` HitResult))
  (bind _returnvalue (message `/Game/CombatSystem/Blueprints/Interfaces/BPI_Combat.CanReceiveDamage?` _hitactor))
  (if _returnvalue
    (`GameplayStatics.ApplyPointDamage` _hitactor (`self.GetDamage`) (`self.GetActorForwardVector` (`self.GetOwner`)) HitResult (`self.GetInstigatorController`) self)))

(event `self.RightFootCollisionComponent.OnHit`
  (params (HitResult :type "HitResult Structure"))
  (bind (_bblockinghit _binitialoverlap _time _distance _location _impactpoint _normal _impactnormal _physmat _hitactor) (`GameplayStatics.BreakHitResult` HitResult))
  (bind _returnvalue (message `/Game/CombatSystem/Blueprints/Interfaces/BPI_Combat.CanReceiveDamage?` _hitactor))
  (if _returnvalue
    (`GameplayStatics.ApplyPointDamage` _hitactor (`self.GetDamage`) (`self.GetActorForwardVector` (`self.GetOwner`)) HitResult (`self.GetInstigatorController`) self)))

(fn `ActivateCollision`
  (params (CollisionPart :type "/Game/CombatSystem/Blueprints/Enums/E_CollisionPart Enum" :default "NewEnumerator0"))
  (switch `/Game/CombatSystem/Blueprints/Enums/E_CollisionPart` CollisionPart
    (:`NewEnumerator0`
      (`/Game/CombatSystem/Blueprints/Components/BP_CollisionComponent.ActivateCollision` (`self.MainWeaponCollisionComponent`)))
    (:`NewEnumerator1`
      (`/Game/CombatSystem/Blueprints/Components/BP_CollisionComponent.ActivateCollision` (`self.OffHandWeaponCollisionComponent`)))
    (:`NewEnumerator2`
      (`/Game/CombatSystem/Blueprints/Components/BP_CollisionComponent.ActivateCollision` (`self.RightFootCollisionComponent`)))))

(fn `AttachOffHandWeapon`
  (params (Socket :type Name))
  (`SceneComponent.K2_AttachToComponent` (`self.OffHandWeaponMesh`) (`Character.Mesh` (cast `Character` (`self.GetOwner`) :!pure true)) Socket "SnapToTarget" "SnapToTarget" "SnapToTarget" true))

(fn `DeactivateCollision`
  (params (CollisionPart :type "/Game/CombatSystem/Blueprints/Enums/E_CollisionPart Enum" :default "NewEnumerator0"))
  (switch `/Game/CombatSystem/Blueprints/Enums/E_CollisionPart` CollisionPart
    (:`NewEnumerator0`
      (`/Game/CombatSystem/Blueprints/Components/BP_CollisionComponent.DeactivateCollision` (`self.MainWeaponCollisionComponent`)))
    (:`NewEnumerator1`
      (`/Game/CombatSystem/Blueprints/Components/BP_CollisionComponent.DeactivateCollision` (`self.OffHandWeaponCollisionComponent`)))
    (:`NewEnumerator2`
      (`/Game/CombatSystem/Blueprints/Components/BP_CollisionComponent.DeactivateCollision` (`self.RightFootCollisionComponent`)))))

(fn `OnEquipped`
  (bind _returnvalue (`self.GetOwner`))
  (`parent.OnEquipped`)
  (`/Game/CombatSystem/Blueprints/Components/BP_CollisionComponent.SetCollisionMesh` (`self.OffHandWeaponCollisionComponent`) (`self.OffHandWeaponMesh`))
  (`/Game/CombatSystem/Blueprints/Components/BP_CollisionComponent.SetCollisionMesh` (`self.RightFootCollisionComponent`) (`Character.Mesh` (cast `Character` (`self.GetOwner`) :!pure true)))
  (`self.AttachOffHandWeapon` (select `bool` (`/Game/CombatSystem/Blueprints/Components/BP_CombatComponent.IsCombatEnabled?` (`self.CombatComponent`)) :`false` (`self.SecondWeaponAttachSocket`) :`true` (`self.SecondWeaponHandSocket`)))
  (`/Game/CombatSystem/Blueprints/Components/BP_CollisionComponent.AddActorToIgnore` (`self.OffHandWeaponCollisionComponent`) _returnvalue)
  (`/Game/CombatSystem/Blueprints/Components/BP_CollisionComponent.AddActorToIgnore` (`self.RightFootCollisionComponent`) _returnvalue))

(fn `UserConstructionScript`
  (`parent.UserConstructionScript`))