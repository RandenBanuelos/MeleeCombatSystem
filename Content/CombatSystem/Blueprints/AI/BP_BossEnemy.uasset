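; Boss enemy that extends a parent AI character with a melee weapon and an on-screen health bar.
; The bar binds to the stats component at BeginPlay, follows target validity for visibility, and is removed on death.
; Weapon collision hits deal stat-based point damage to actors that accept it.
; The weapon mesh swaps sockets when combat toggles and switches to physics simulation on death.
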(event `self.ReceiveBeginPlay`
  (`parent.ReceiveBeginPlay`)
  (`/Game/CombatSystem/Blueprints/Components/BP_CollisionComponent.SetCollisionMesh` (`self.MainWeaponCollisionComponent`) (`self.WeaponMesh`))
  (bind _returnvalue (`|CreateWidget` "/Game/CombatSystem/UI/WB_BossHealthBar.WB_BossHealthBar_C" (`GameplayStatics.GetPlayerController` 0)))
  (bind _output_get (set `self.BossHealthUI` _returnvalue))
  (`/Game/CombatSystem/UI/WB_BossHealthBar.Initialize` _output_get (`self.StatsComponent`))
  (`UserWidget.AddToViewport` _output_get 0))

(event `self.OnTargeted`
  (params (`bIsTargeted?` :type Boolean))
  (`parent.OnTargeted` `bIsTargeted?`))

(event `self.MainWeaponCollisionComponent.OnHit`
  (params (HitResult :type "HitResult Structure"))
  (bind (_bblockinghit _binitialoverlap _time _distance _location _impactpoint _normal _impactnormal _physmat _hitactor) (`GameplayStatics.BreakHitResult` HitResult))
  (bind _returnvalue (message `/Game/CombatSystem/Blueprints/Interfaces/BPI_Combat.CanReceiveDamage?` _hitactor))
  (if _returnvalue
    (`GameplayStatics.ApplyPointDamage` _hitactor (`/Game/CombatSystem/Blueprints/Components/BP_StatsComponent.GetCurrentStatValue` (`self.StatsComponent`) "NewEnumerator4") (`self.GetActorForwardVector` (`self.GetOwner`)) HitResult (`self.GetController`) self (`self.DamageTypeClass`))))

(event `SimulateWeaponPhysics`
  (bind _weaponmesh (`self.WeaponMesh`))
  (`PrimitiveComponent.SetCollisionProfileName` _weaponmesh "PhysicsActor" true)
  (`PrimitiveComponent.SetSimulatePhysics` _weaponmesh true))

(event `self.PerformDeath`
  (`parent.PerformDeath`)
  (`self.SimulateWeaponPhysics`)
  (`self.SetBossHealthVisibility` false)
  (`Widget.RemoveFromParent` (`self.BossHealthUI`)))

(event `self.CombatComponent.OnCombatToggled`
  (params (`bIsCombatEnabled?` :type Boolean))
  (`SceneComponent.K2_AttachToComponent` (`self.WeaponMesh`) (`self.Mesh`) (select `bool` `bIsCombatEnabled?` :`false` (`self.AttachSocketName`) :`true` (`self.WeaponHandSocketName`)) "SnapToTarget" "SnapToTarget" "SnapToTarget" true))

(event `SetBossHealthVisibility`
  (params (`bVisible?` :type Boolean))
  (bind _bosshealthui (`self.BossHealthUI`)
    (:`then`
      (`Widget.SetVisibility` _bosshealthui (select `bool` `bVisible?` :`false` "Hidden" :`true` "Visible" :!type "ESlateVisibility Enum")))
    (:`else`)))

(event `self.OnTargetSet`
  (params (SensedActor :type "Actor Object Reference"))
  (`parent.OnTargetSet` SensedActor)
  (`self.SetBossHealthVisibility` (`KismetSystemLibrary.IsValid` SensedActor)))

(fn `UserConstructionScript`
  (`parent.UserConstructionScript`))