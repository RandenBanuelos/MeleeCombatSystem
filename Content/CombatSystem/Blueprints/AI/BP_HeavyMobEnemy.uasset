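; BP_HeavyMobEnemy is a heavy melee enemy that carries a physical weapon mesh.
; Weapon collision hits apply point damage from its stats component to actors that can receive damage.
; Toggling combat moves the weapon between hand and holster sockets, and death switches it to simulated physics.
; A health bar widget fed by the enemy's stats is created at BeginPlay and shown only while the enemy is targeted.
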(event `self.ReceiveBeginPlay`
  (`parent.ReceiveBeginPlay`)
  (`/Game/CombatSystem/Blueprints/Components/BP_CollisionComponent.SetCollisionMesh` (`self.MainWeaponCollisionComponent`) (`self.WeaponMesh`))
  (bind _returnvalue (`|CreateWidget` "/Game/CombatSystem/UI/WB_HealthBar.WB_HealthBar_C" (`GameplayStatics.GetPlayerController` 0) (`self.StatsComponent`) false))
  (`WidgetComponent.SetWidget` (`self.HealthBarWidget`) _returnvalue))

(event `self.OnTargeted`
  (params (`bIsTargeted?` :type Boolean))
  (`parent.OnTargeted` `bIsTargeted?`)
  (`SceneComponent.SetVisibility` (`self.HealthBarWidget`) `bIsTargeted?` false))

(event `self.MainWeaponCollisionComponent.OnHit`
  (params (HitResult :type "HitResult Structure"))
  (bind (_bblockinghit _binitialoverlap _time _distance _location _impactpoint _normal _impactnormal _physmat _hitactor) (`GameplayStatics.BreakHitResult` HitResult))
  (bind _returnvalue (message `/Game/CombatSystem/Blueprints/Interfaces/BPI_Combat.CanReceiveDamage?` _hitactor))
  (if _returnvalue
    (`GameplayStatics.ApplyPointDamage` _hitactor (`/Game/CombatSystem/Blueprints/Components/BP_StatsComponent.GetCurrentStatValue` (`self.StatsComponent`) "NewEnumerator4") (`self.GetActorForwardVector` (`self.GetOwner`)) HitResult (`self.GetController`) self (`self.DamageTypeClass`))))

(event `SimulateWeaponPhysics`
  (bind _weaponmesh (`self.WeaponMesh`))
  (`PrimitiveComponent.SetCollisionProfileName` _weaponmesh "PhysicsActor" true)
  (`PrimitiveComponent.SetSimulatePhysics` _weaponmesh true))

(event `self.PerformDeath`
  (`parent.PerformDeath`)
  (`self.SimulateWeaponPhysics`))

(event `self.CombatComponent.OnCombatToggled`
  (params (`bIsCombatEnabled?` :type Boolean))
  (`SceneComponent.K2_AttachToComponent` (`self.WeaponMesh`) (`self.Mesh`) (select `bool` `bIsCombatEnabled?` :`false` (`self.AttachSocketName`) :`true` (`self.WeaponHandSocketName`)) "SnapToTarget" "SnapToTarget" "SnapToTarget" true))

(fn `UserConstructionScript`
  (`parent.UserConstructionScript`))