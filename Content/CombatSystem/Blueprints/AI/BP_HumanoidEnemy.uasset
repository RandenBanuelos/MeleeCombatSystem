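; BP_HumanoidEnemy is a humanoid enemy in the combat system that shows a health bar while it is targeted.
; On BeginPlay it creates a WB_HealthBar bound to its own StatsComponent instead of the player's and assigns it to the HealthBarWidget component.
; The OnTargeted event toggles that component's visibility, and all overridden events also run the parent class logic.
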(event `self.ReceiveBeginPlay`
  (`parent.ReceiveBeginPlay`)
  (bind _returnvalue (`|CreateWidget` "/Game/CombatSystem/UI/WB_HealthBar.WB_HealthBar_C" (`GameplayStatics.GetPlayerController` 0) (`self.StatsComponent`) false))
  (`WidgetComponent.SetWidget` (`self.HealthBarWidget`) _returnvalue))

(event `/Game/CombatSystem/Blueprints/Interfaces/BPI_Targeting.OnTargeted`
  (params (`bIsTargeted?` :type Boolean))
  (`parent.OnTargeted` `bIsTargeted?`)
  (`SceneComponent.SetVisibility` (`self.HealthBarWidget`) `bIsTargeted?` false))

(fn `UserConstructionScript`
  (`parent.UserConstructionScript`))