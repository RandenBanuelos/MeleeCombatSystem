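; Anim notify that toggles combat mode on a BP_CombatCharacter at a frame in an animation, such as a draw or sheathe.
; It gets the main weapon from the owner's BP_CombatComponent and, if valid, attaches it to its hand socket or its stowed attach socket based on the EnableCombat flag.
; It then sets the component's combat enabled state to the same flag.
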(fn `Received_Notify`
  (params (MeshComp :type "SkeletalMeshComponent Object Reference") (Animation :type "AnimSequenceBase Object Reference") (EventReference :type "AnimNotifyEventReference Structure (by ref)"))
  (returns (ReturnValue :type Boolean))
  (bind _asbp_combat_character (cast `/Game/CombatSystem/Blueprints/BP_CombatCharacter` (`ActorComponent.GetOwner` MeshComp)))
  (bind _returnvalue (`Actor.GetComponentByClass` _asbp_combat_character "/Game/CombatSystem/Blueprints/Components/BP_CombatComponent.BP_CombatComponent_C"))
  (bind _mainweapon (`/Game/CombatSystem/Blueprints/Components/BP_CombatComponent.GetMainWeapon` _returnvalue))
  (`/Engine/EditorBlueprintResources/StandardMacros.IsValid` _mainweapon
    (:`Is Valid`
      (`/Game/CombatSystem/Blueprints/Actors/BP_BaseEquippable.AttachActor` _mainweapon (select `bool` (`self.bEnableCombat?`) :`false` (`/Game/CombatSystem/Blueprints/Actors/BP_BaseEquippable.AttachSocketName` _mainweapon) :`true` (`/Game/CombatSystem/Blueprints/Actors/BP_BaseWeapon.HandSocketName` _mainweapon)))
      (`/Game/CombatSystem/Blueprints/Components/BP_CombatComponent.SetCombatEnabled` _returnvalue (`self.bEnableCombat?`))
      (return true))))