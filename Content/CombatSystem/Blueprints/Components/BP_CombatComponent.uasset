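; BP_CombatComponent is an actor component that holds a character's main weapon, combat state and attack tracking values.
; Setting a new main weapon first unequips and destroys the current one, if valid, then stores the replacement.
; Toggling combat stores the flag and forwards it to the owning Character's mesh anim instance through an update message.
; ResetAttack clears the attack count and the saved-attack flag.
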(fn `GetMainWeapon`
  (returns (MainWeapon :type "/Game/CombatSystem/Blueprints/Actors/BP_BaseWeapon Object Reference"))
  (return (`self.MainWeapon`)))

(fn `IsCombatEnabled?`
  (returns (ReturnValue :type Boolean))
  (return (`self.bCombatEnabled?`)))

(fn `ResetAttack`
  (set `self.AttackCount` 0)
  (set `self.bIsAttackSaved?` false))

(fn `SetCombatEnabled`
  (params (`bCombatEnabled?` :type Boolean))
  (bind _output_get (set `self.bCombatEnabled?` `bCombatEnabled?`))
  (message `/Game/CombatSystem/Blueprints/Interfaces/BPI_AnimInstance.UpdateCombatEnabled` (`SkeletalMeshComponent.GetAnimInstance` (`Character.Mesh` (cast `Character` (`self.GetOwner`) :!pure true))) _output_get))

(fn `SetMainWeapon`
  (params (NewWeapon :type "/Game/CombatSystem/Blueprints/Actors/BP_BaseWeapon Object Reference"))
  (`|ExecutionSequence`
    (:`then_0`
      (bind _mainweapon (`self.MainWeapon`)
        (:`then`
          (`/Game/CombatSystem/Blueprints/Actors/BP_BaseEquippable.OnUnequipped` _mainweapon)
          (`Actor.K2_DestroyActor` _mainweapon))
        (:`else`)))
    (:`then_1`
      (set `self.MainWeapon` NewWeapon))))