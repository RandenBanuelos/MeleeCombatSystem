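; BP_StatsComponent is a combat component that stores an actor's stats and applies damage to them.
; A BaseStats map holds base and max values per stat, and InitializeStats copies each base value into the CurrentStats map.
; Modifications to current values are clamped between zero and max, while direct setters are unclamped.
; TakeDamage reduces one stat, presumably health, and switches the owner's BP_StateManager state when it reaches zero.
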(fn `GetBaseStatValue`
  (params (Stat :type "/Game/CombatSystem/Blueprints/Enums/E_Stat Enum" :default "NewEnumerator0"))
  (returns (BaseValue :type "Float (double-precision)"))
  (return (break `/Game/CombatSystem/Blueprints/Structs/F_BaseStat` (`BlueprintMapLibrary.Map_Find` (`self.BaseStats`) Stat))))

(fn `GetCurrentStatValue`
  (params (Stat :type "/Game/CombatSystem/Blueprints/Enums/E_Stat Enum" :default "NewEnumerator0"))
  (returns (Value :type "Float (double-precision)"))
  (return (`BlueprintMapLibrary.Map_Find` (`self.CurrentStats`) Stat)))

(fn `GetMaxStatValue`
  (params (Stat :type "/Game/CombatSystem/Blueprints/Enums/E_Stat Enum" :default "NewEnumerator0"))
  (returns (MaxValue :type "Float (double-precision)"))
  (return (`.MaxValue_5_507EF67D41D4E0724071F1A26380AC60` (break `/Game/CombatSystem/Blueprints/Structs/F_BaseStat` (`BlueprintMapLibrary.Map_Find` (`self.BaseStats`) Stat)))))

(fn `InitializeStats`
  (bind _basestats (`self.BaseStats`))
  (bind _keys (`BlueprintMapLibrary.Map_Keys` _basestats))
  (for _array_element _keys
    (`self.SetCurrentStatValue` _array_element (break `/Game/CombatSystem/Blueprints/Structs/F_BaseStat` (`BlueprintMapLibrary.Map_Find` _basestats _array_element)))))

(fn `ModifyCurrentStatValue`
  (params (Stat :type "/Game/CombatSystem/Blueprints/Enums/E_Stat Enum" :default "NewEnumerator0") (Value :type "Float (double-precision)"))
  (locals (L_Value :type "Float (double-precision)"))
  (bind _stat (`local.Stat`))
  (if (!= Value 0.0)
    (bind _output_get (set `local.L_Value` (+ (`self.GetCurrentStatValue` Stat) Value)))
    (bind _output_get_2 (set `local.L_Value` (`KismetMathLibrary.FClamp` _output_get 0.0 (`self.GetMaxStatValue` _stat))))
    (`self.SetCurrentStatValue` _stat _output_get_2)))

(fn `SetBaseStatValue`
  (params (Stat :type "/Game/CombatSystem/Blueprints/Enums/E_Stat Enum" :default "NewEnumerator0") (Value :type "Float (double-precision)"))
  (bind _basestats (`self.BaseStats`))
  (bind _structout (setmembers `/Game/CombatSystem/Blueprints/Structs/F_BaseStat` :`StructRef` (`BlueprintMapLibrary.Map_Find` _basestats Stat) :`BaseValue` Value))
  (`BlueprintMapLibrary.Map_Add` _basestats (`local.Stat`) _structout))

(fn `SetCurrentStatValue`
  (params (Stat :type "/Game/CombatSystem/Blueprints/Enums/E_Stat Enum" :default "NewEnumerator0") (Value :type "Float (double-precision)"))
  (`BlueprintMapLibrary.Map_Add` (`self.CurrentStats`) Stat Value))

(fn `SetMaxStatValue`
  (params (Stat :type "/Game/CombatSystem/Blueprints/Enums/E_Stat Enum" :default "NewEnumerator0") (Value :type "Float (double-precision)"))
  (bind _basestats (`self.BaseStats`))
  (bind _structout (setmembers `/Game/CombatSystem/Blueprints/Structs/F_BaseStat` :`StructRef` (`BlueprintMapLibrary.Map_Find` _basestats Stat) :`MaxValue` Value))
  (`BlueprintMapLibrary.Map_Add` _basestats (`local.Stat`) _structout))

(fn `TakeDamage`
  (params (InDamage :type "Float (double-precision)"))
  (`self.ModifyCurrentStatValue` "NewEnumerator1" (* InDamage -1.0))
  (if (<= (`self.GetCurrentStatValue` "NewEnumerator1") 0.0)
    (`/Game/CombatSystem/Blueprints/Components/BP_StateManager.SetState` (`Actor.GetComponentByClass` (`self.GetOwner`) "/Game/CombatSystem/Blueprints/Components/BP_StateManager.BP_StateManager_C") "NewEnumerator4")))